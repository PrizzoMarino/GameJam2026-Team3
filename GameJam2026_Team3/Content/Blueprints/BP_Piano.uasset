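; BP_Piano is a scripted falling-piano trap that can kill the first-person player.
; TriggerBox fires once on player overlap, playing a rope sound, spawning a moving BP_Car, then enabling physics on the meshes in staggered steps with a crash sound.
; A separate Box handles death once on player overlap, independently of that sequence: it fades the camera out, shows the WBP_OldHag widget and opens Map1.
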(event OnComponentBeginOverlap(Box)
  (params (OverlappedComponent :type Primitive%20Component%20Object%20Reference) (OtherActor :type Actor%20Object%20Reference) (OtherComp :type Primitive%20Component%20Object%20Reference) (OtherBodyIndex :type Integer) (bFromSweep :type Boolean) (SweepResult :type Hit%20Result%20Structure%20%28by%20ref%29))
  (bind _asbp_first_person_character (Utilities|Casting|CastToBP_FirstPersonCharacter OtherActor))
  (if (not (Variables|Default|GethasDied))
    (CameraFades|StartCameraFade :self (Variables|/Script/Engine.PlayerController|GetPlayerCameraManager (Pawn|GetLocalViewingPlayerController _asbp_first_person_character)) :ToAlpha 1.0 :Duration 0.2 :bHoldWhenFinished true)
    (Variables|Default|SethasDied true)
    (Utilities|FlowControl|Delay 0.5)
    (bind _returnvalue (UserInterface|CreateWidget "/Game/Blueprints/WBP_OldHag.WBP_OldHag_C"))
    (UserInterface|Viewport|AddtoViewport _returnvalue 0)
    (Game|OpenLevel(byName) "Map1")))

(event OnComponentBeginOverlap(TriggerBox)
  (params (OverlappedComponent :type Primitive%20Component%20Object%20Reference) (OtherActor :type Actor%20Object%20Reference) (OtherComp :type Primitive%20Component%20Object%20Reference) (OtherBodyIndex :type Integer) (bFromSweep :type Boolean) (SweepResult :type Hit%20Result%20Structure%20%28by%20ref%29))
  (Utilities|Casting|CastToBP_FirstPersonCharacter OtherActor)
  (if (not (Variables|Default|GethasTriggered))
    (Variables|Default|SethasTriggered true)
    (Audio|PlaySoundatLocation "/Game/Audio/Rope_sound.Rope_sound" (Variables|/Script/Engine.SceneComponent|GetRelativeLocation (Variables|Default|GetStaticMesh)) "0, 0, 0" 1.0 1.0 0.0 0 0 0 0)
    (Utilities|FlowControl|Delay 1.0)
    (bind _returnvalue (Game|SpawnActorfromClass "/Game/Blueprints/BP_Car.BP_Car_C" (Math|Transform|MakeTransform "-620.000000,3160.000000,40.000000" "0, 0, 0" "1.000000,1.000000,1.000000") "Undefined" "MultiplyWithRoot" 0 0))
    (Default|CarMove _returnvalue)
    (Utilities|FlowControl|Delay 2.0)
    (Physics|SetSimulatePhysics (Variables|Default|GetStaticMesh) true)
    (Physics|SetEnableGravity (Variables|Default|GetStaticMesh) true)
    (Audio|PlaySoundatLocation "/Game/Audio/falling_piano_sound.falling_piano_sound" (Variables|/Script/Engine.SceneComponent|GetRelativeLocation (Variables|Default|GetStaticMesh)) "0, 0, 0" 1.0 1.0 0.0 0 0 0 0)
    (Utilities|FlowControl|Delay 0.2)
    (Physics|SetSimulatePhysics (Variables|Default|GetStaticMesh1) true)
    (Physics|SetSimulatePhysics (Variables|Default|GetStaticMesh2) true)))

(event EventBeginPlay)

(event Collision|EventActorBeginOverlap
  (params (OtherActor :type Actor%20Object%20Reference)))

(event EventTick
  (params (DeltaSeconds :type Float%20%28single-precision%29)))

(fn ConstructionScript)