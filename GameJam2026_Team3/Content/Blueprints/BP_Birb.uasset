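; BP_Birb is a hazard actor that ends the player's run by reloading or switching to Map1 on touch.
; When its Box overlaps BP_FirstPersonCharacter, it fades the camera out, holds it, waits briefly, then opens Map1.
; A BirbSwarm event spawns twenty more BP_Birb actors at random directions on a fixed-radius sphere around the supplied actor's location.
; The Blueprint itself contains no movement logic.
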(event OnComponentBeginOverlap(Box)
  (params (OverlappedComponent :type Primitive%20Component%20Object%20Reference) (OtherActor :type Actor%20Object%20Reference) (OtherComp :type Primitive%20Component%20Object%20Reference) (OtherBodyIndex :type Integer) (bFromSweep :type Boolean) (SweepResult :type Hit%20Result%20Structure%20%28by%20ref%29))
  (bind _asbp_first_person_character (Utilities|Casting|CastToBP_FirstPersonCharacter OtherActor))
  (CameraFades|StartCameraFade :self (Variables|/Script/Engine.PlayerController|GetPlayerCameraManager (Pawn|GetLocalViewingPlayerController _asbp_first_person_character)) :ToAlpha 1.0 :Duration 0.2 :bHoldWhenFinished true)
  (Utilities|FlowControl|Delay 2.0)
  (Game|OpenLevel(byName) "Map1"))

(event Custom|BirbSwarm
  (params (PlayerLocation :type BP%20First%20Person%20Character%20Object%20Reference))
  (for _index (range 0 19)
    (Game|SpawnActorfromClass "BP_Birb_C" (Math|Conversions|ToTransform(Vector) (+ (* (Math|Random|RandomUnitVector) 1000) (Transformation|GetActorLocation PlayerLocation))) "Undefined" "MultiplyWithRoot" 0 0)))

(event EventBeginPlay)

(event Collision|EventActorBeginOverlap
  (params (OtherActor :type Actor%20Object%20Reference)))

(event EventTick
  (params (DeltaSeconds :type Float%20%28single-precision%29)))

(fn ConstructionScript)