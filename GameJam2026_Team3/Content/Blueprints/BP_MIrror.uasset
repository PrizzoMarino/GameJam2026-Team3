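; BP_MIrror is a breakable mirror that ends the current scene by loading Map1.
; MirrorBreak fires once, swapping in the broken mesh, playing a sound and adding an offset, rotated mesh component.
; That component is launched toward the supplied player position with extra upward velocity.
; After short delays, the player's camera fades out and holds, then the level opens.
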(event Custom|MirrorBreak
  (params (PlayerPos :type Vector) (Player :type BP%20First%20Person%20Character%20Object%20Reference))
  (bind _mirror (Variables|Default|GetMirror))
  (bind _returnvalue (Transformation|GetRelativeTransform _mirror))
  (if (not (Variables|Default|GetbhasBroken))
    (Variables|Default|SetbhasBroken true)
    (Components|StaticMesh|SetStaticMesh _mirror "/Game/SM/Broken_mirror.Broken_mirror")
    (Audio|PlaySoundatLocation 0 (Transformation|GetWorldLocation _mirror) "0, 0, 0" 1.0 1.0 0.0 0 0 0 0)
    (bind _returnvalue_2 (AddComponent|AddStaticMeshComponent false (Math|Transform|MakeTransform (Math|Vector|MakeVector (- (.x (.location _returnvalue)) 4e+01) (.y (.location _returnvalue)) (.z (.location _returnvalue))) (Math|Rotator|MakeRotator (.roll (.rotation _returnvalue)) (+ (.pitch (.rotation _returnvalue)) 9e+01) (.yaw (.rotation _returnvalue))) "1.000000,1.000000,1.000000")))
    (Physics|SetPhysicsLinearVelocity _returnvalue_2 (Math|Vector|MakeVector (.x (* (Math|Vector|Normalize (- PlayerPos (Transformation|GetWorldLocation _returnvalue_2))) 1e+03)) (.y (* (Math|Vector|Normalize (- PlayerPos (Transformation|GetWorldLocation _returnvalue_2))) 1e+03)) (+ (.z (* (Math|Vector|Normalize (- PlayerPos (Transformation|GetWorldLocation _returnvalue_2))) 1e+03)) 4.5e+02)) false "None")
    (Utilities|FlowControl|Delay 0.3)
    (CameraFades|StartCameraFade :self (Variables|/Script/Engine.PlayerController|GetPlayerCameraManager (Pawn|GetLocalViewingPlayerController Player)) :ToAlpha 1.0 :Duration 0.2 :bHoldWhenFinished true)
    (Utilities|FlowControl|Delay 2.0)
    (Game|OpenLevel(byName) "Map1")))

(event EventBeginPlay)

(event Collision|EventActorBeginOverlap
  (params (OtherActor :type Actor%20Object%20Reference)))

(event EventTick
  (params (DeltaSeconds :type Float%20%28single-precision%29)))

(fn ConstructionScript)